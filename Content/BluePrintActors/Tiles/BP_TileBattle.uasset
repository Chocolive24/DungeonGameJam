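; BP_TileBattle is a tile that starts a battle when the player enters its collision.
; On BeginPlay it caches the battle and tiles managers and records the world positions of its Tiles' collision spheres.
; On player entry, after the parent logic, it passes tiles and positions to the tiles manager's GetAllRoomTiles, then has the battle manager instantiate its Enemies and start the battle.
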(event `self.ReceiveBeginPlay`
  (bind _returnvalue (`GameplayStatics.GetActorOfClass` "/Game/BluePrintActors/Managers/BP_BattleManager.BP_BattleManager_C"))
  (set `self.BattleManagerRef` _returnvalue)
  (bind _returnvalue_2 (`GameplayStatics.GetActorOfClass` "/Game/BluePrintActors/Managers/BP_TilesManager.BP_TilesManager_C"))
  (set `self.BP_TilesManagerRef` _returnvalue_2)
  (for _array_element (`self.Tiles`)
    (`KismetArrayLibrary.Array_Add` (`self.TilesPosition`) (`SceneComponent.K2_GetComponentLocation` (`/Game/BluePrintActors/Tiles/BP_Tile.CollisonSphere` _array_element)))
    (for _ (`self.TilesPosition`)
      _)))

(event `self.EnterPlayerCollision`
  (bind _battlemanagerref (`self.BattleManagerRef`))
  (`parent.EnterPlayerCollision`)
  (`/Game/BluePrintActors/Managers/BP_TilesManager.GetAllRoomTiles` (`self.BP_TilesManagerRef`) (`self.TilesPosition`) (`self.Tiles`))
  (`/Game/BluePrintActors/Managers/BP_BattleManager.InstantiateEnemies` _battlemanagerref (`self.Enemies`))
  (`/Game/BluePrintActors/Managers/BP_BattleManager.StartBattle` _battlemanagerref))

(event `self.ExitPlayerCollision`
  (`parent.ExitPlayerCollision`))

(fn `UserConstructionScript`
  (`parent.UserConstructionScript`))