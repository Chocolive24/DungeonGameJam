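; Player pawn for a turn-based tile game that moves between BP_Tile actors, with health and action points that start at maximum.
; Forward input line-traces along its facing, notifies the old and new tiles of exit and enter, and snaps the capsule to the hit tile's sphere.
; Side input yaws it in 90-degree steps.
; Events apply damage, spend action points and refill them at turn start; a debug key possesses a spawned DefaultPawn.
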(event `Key|One`
  (params (Key :type "Key Structure"))
  ;[1 1 1] Debug Pawn
  (:`Pressed`
    (bind _returnvalue (`|SpawnActorFromClass` "/Script/Engine.DefaultPawn" (`self.GetTransform`) "Undefined" "OverrideRootScale" null null))
    (`Controller.Possess` (`GameplayStatics.GetPlayerController` 0) _returnvalue)))

(event `self.ReceiveBeginPlay`
  (set `self.CurrentHealthPoints` (`self.MaxHealthPoints`))
  (set `self.CurrentActionPoints` (`self.MaxActionPoints`))
  (`SceneComponent.K2_SetWorldLocation` (`self.CapsuleComponent`) (0.0 0.0 30.0) false false))

(event `ForwardMove`
  (params (InputAxisValue :type Integer))
  (bind _capsulecomponent (`self.CapsuleComponent`))
  (bind _bp_tileref (`self.BP_TileRef`))
  (bind _returnvalue (`SceneComponent.K2_GetComponentLocation` _capsulecomponent))
  (bind _returnvalue_2 (+ (* (* (`SceneComponent.GetForwardVector` _capsulecomponent) InputAxisValue) (1000.0 1000.0 0.0)) _returnvalue))
  ;[1 1 1] Forward Movement
  (`KismetSystemLibrary.PrintString` (`KismetStringLibrary.Conv_VectorToString` _returnvalue_2))
  (bind _outhit (`KismetSystemLibrary.LineTraceSingle` :`Start` _returnvalue :`End` _returnvalue_2 :`TraceChannel` "TraceTypeQuery1" :`DrawDebugType` "Persistent"))
  (`/Engine/EditorBlueprintResources/StandardMacros.IsValid` _bp_tileref
    (:`Is Valid`
      (`/Game/BluePrintActors/Tiles/BP_Tile.ExitPlayerCollision` _bp_tileref))
    (:`Is Not Valid`
      _))
  (bind _asbp_tile (cast `/Game/BluePrintActors/Tiles/BP_Tile` (`.HitActor` (`GameplayStatics.BreakHitResult` _outhit))))
  (set `self.BP_TileRef` _asbp_tile)
  (`/Game/BluePrintActors/Tiles/BP_Tile.EnterPlayerCollision` _asbp_tile)
  (`SceneComponent.K2_SetWorldLocation` (`self.CapsuleComponent`) (`SceneComponent.K2_GetComponentLocation` (`/Game/BluePrintActors/Tiles/BP_Tile.CollisonSphere` _asbp_tile)) true false)
  (`KismetSystemLibrary.PrintString` (`KismetStringLibrary.Conv_VectorToString` (`SceneComponent.K2_GetComponentLocation` (`self.CapsuleComponent`)))))

(event `SideMove`
  (params (InputAxisValue :type Integer))
  ;[1 1 1] Side Rotation Movement Logic
  (`SceneComponent.K2_SetWorldRotation` (`self.CapsuleComponent`) (`KismetMathLibrary.MakeRotator` (.roll (`SceneComponent.K2_GetComponentRotation` (`self.CapsuleComponent`))) (.pitch (`SceneComponent.K2_GetComponentRotation` (`self.CapsuleComponent`))) (`KismetMathLibrary.Conv_IntToDouble` (+ (* InputAxisValue 90) (`KismetMathLibrary.FTrunc` (.yaw (`SceneComponent.K2_GetComponentRotation` (`self.CapsuleComponent`))))))) false false))

(event `TakeDamage`
  (params (Damage :type Integer))
  ;[1 1 1] Take Damage Logic
  (bind _output_get (set `self.CurrentHealthPoints` (- (`self.CurrentHealthPoints`) Damage))))

(event `RemoveActionPoints`
  (params (nbrToRemove :type Integer))
  ;[1 1 1] Remove Action Points Logic
  (bind _output_get (set `self.CurrentActionPoints` (- (`self.CurrentActionPoints`) nbrToRemove))))

(event `StartTurn`
  (bind _output_get (set `self.CurrentActionPoints` (`self.MaxActionPoints`)))
  (`WidgetBlueprintLibrary.SetInputMode_GameAndUIEx` (`GameplayStatics.GetPlayerController` 0) null)
  (`KismetSystemLibrary.PrintString` (`KismetStringLibrary.Conv_IntToString` _output_get)))

(fn `UserConstructionScript`)