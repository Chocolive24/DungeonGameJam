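; Player controller that routes forward and side inputs to BP_Player movement, or to a combo buffer while the player is in battle.
; In battle, each press costs an action point and retriggers a cooldown delay, after which the buffered keys are printed and cleared, with no combo effects yet.
; The EndTurn input, in battle only, switches to UI-only input and advances the turn through the BP_BattleManager found at BeginPlay.
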(event `self.ReceiveBeginPlay`
  ;[1 1 1] Begin Play Logic
  (bind _returnvalue (`GameplayStatics.GetActorOfClass` "/Game/BluePrintActors/Managers/BP_BattleManager.BP_BattleManager_C"))
  (set `self.BattleManagerRef` _returnvalue))

(event `PerformForwardInput`
  (params (`Axis Value` :type Integer) (`Key Pressed` :type "Key Structure" :default "None"))
  ;[1 1 1] ForwardInputs
  (bind _asbp_player (cast `/Game/BluePrintActors/Player/BP_Player_Auto1` (`GameplayStatics.GetPlayerCharacter` 0)))
  (if (`/Game/BluePrintActors/Player/BP_Player_Auto1.IsInBattle?` _asbp_player)
    (`self.AddKeyToCombo` `Key Pressed`)
    (`/Game/BluePrintActors/Player/BP_Player_Auto1.RemoveActionPoints` _asbp_player 1)
    (else
      (`/Game/BluePrintActors/Player/BP_Player_Auto1.ForwardMove` _asbp_player `Axis Value`))))

(event `InputAction|ForwardMovementUp`
  (params (Key :type "Key Structure"))
  ;[1 1 1] ForwardInputs
  (:`Pressed`
    (`self.PerformForwardInput` 1 Key)))

(event `InputAction|ForwardMovementDown`
  (params (Key :type "Key Structure"))
  ;[1 1 1] ForwardInputs
  (:`Pressed`
    (`self.PerformForwardInput` -1 Key)))

(event `PerformSideInput`
  (params (AxisValue :type Integer) (KeyPressed :type "Key Structure" :default "None"))
  ;[1 1 1] SideInputs
  (bind _asbp_player (cast `/Game/BluePrintActors/Player/BP_Player_Auto1` (`GameplayStatics.GetPlayerCharacter` 0)))
  (if (`/Game/BluePrintActors/Player/BP_Player_Auto1.IsInBattle?` _asbp_player)
    (`self.AddKeyToCombo` KeyPressed)
    (`/Game/BluePrintActors/Player/BP_Player_Auto1.RemoveActionPoints` _asbp_player 1)
    (else
      (`/Game/BluePrintActors/Player/BP_Player_Auto1.SideMove` _asbp_player AxisValue))))

(event `InputAction|LeftRotation`
  (params (Key :type "Key Structure"))
  ;[1 1 1] SideInputs
  (:`Pressed`
    (`self.PerformSideInput` 1 Key)))

(event `InputAction|RightRotation`
  (params (Key :type "Key Structure"))
  ;[1 1 1] SideInputs
  (:`Pressed`
    (`self.PerformSideInput` -1 Key)))

(event `AddKeyToCombo`
  (params (KeyPressed :type "Key Structure" :default "None"))
  ;[1 1 1] Combo Logic
  (`KismetArrayLibrary.Array_Add` (`self.Inputs`) KeyPressed)
  (set `self.LastInputTime` (`KismetSystemLibrary.GetGameTimeInSeconds`))
  (`self.CheckExecuteCombo`))

(event `CheckExecuteCombo`
  (bind _returnvalue (`KismetArrayLibrary.Array_Length` (`self.Inputs`)))
  ;[1 1 1] Check if must perform combo
  (if (> (mod _returnvalue 4) (`self.InputsLength`))
    (set `self.InputsLength` _returnvalue))
  (`KismetSystemLibrary.RetriggerableDelay` (`self.InputCooldown`))
  (`self.PerformCombo`)
  (`KismetArrayLibrary.Array_Clear` (`self.Inputs`)))

(event `PerformCombo`
  (bind _returnvalue (`GameplayStatics.GetPlayerController` 0))
  ;[1 1 1] Perform Combo Logic
  (`self.DisableInput` _returnvalue null)
  (for (_ _array_index) (`self.Inputs`)
    (`KismetSystemLibrary.PrintString` (`KismetStringLibrary.Conv_IntToString` _array_index))
    (`self.EnableInput` _returnvalue null)))

(event `InputAction|EndTurn`
  (params (Key :type "Key Structure"))
  ;[1 1 1] End Turn Button Logic
  (:`Pressed`
    (bind _asbp_player (cast `/Game/BluePrintActors/Player/BP_Player_Auto1` (`GameplayStatics.GetPlayerCharacter` 0)))
    (if (`/Game/BluePrintActors/Player/BP_Player_Auto1.IsInBattle?` _asbp_player)
      (`WidgetBlueprintLibrary.SetInputMode_UIOnlyEx` (`GameplayStatics.GetPlayerController` 0) null)
      (`/Game/BluePrintActors/Managers/BP_BattleManager.SetNextTurn` (`self.BattleManagerRef`)))))

(fn `UserConstructionScript`)