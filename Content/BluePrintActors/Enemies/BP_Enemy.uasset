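; Turn-based grid enemy that, on StartTurn, computes a tile path to the player, debug-prints it and hands the turn back to BP_BattleManager without moving.
; FindPath is an A*-style search over BP_TilesManager tiles, using Manhattan distances from start and goal as G and H, ordered by SortArray.
; RestructurePath walks previous-tile links to build the route.
; A breadth-first range search (GetAvailableTiles) is unwired; FindPathDijkstra is empty.
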(event `self.ReceiveBeginPlay`
  (bind _returnvalue (`GameplayStatics.GetActorOfClass` "/Game/BluePrintActors/Managers/BP_BattleManager.BP_BattleManager_C"))
  (set `self.BP_BattleManagerRef` _returnvalue)
  (bind _returnvalue_2 (`GameplayStatics.GetActorOfClass` "/Game/BluePrintActors/Managers/BP_TilesManager.BP_TilesManager_C"))
  (set `self.BP_TilesManagerRef` _returnvalue_2)
  (bind _returnvalue_3 (`GameplayStatics.GetActorOfClass` "/Game/BluePrintActors/Player/BP_Player_Auto1.BP_Player_C"))
  (set `self.BP_PlayerRef` _returnvalue_3))

(event `StartTurn`
  (bind _path (`self.FindPath` (`SceneComponent.K2_GetComponentLocation` (`self.Cube`)) (`SceneComponent.K2_GetComponentLocation` (`Character.CapsuleComponent` (`GameplayStatics.GetPlayerCharacter` 0)))))
  (bind _output_get (set `self.Path` _path))
  (for _array_element _output_get
    (`KismetSystemLibrary.PrintString` (`KismetStringLibrary.Conv_VectorToString` _array_element) true true (struct :`G` 0.66 :`B` 1.0 :`A` 1.0) 20.0))
  (`KismetSystemLibrary.PrintString` (`KismetSystemLibrary.GetDisplayName` self))
  (`/Game/BluePrintActors/Managers/BP_BattleManager.SetNextTurn` (`self.BP_BattleManagerRef`))
  (bind _isposavailable_ (`self.IsPositionAvailable` (600.0 -200.0 30.0)))
  (`KismetSystemLibrary.PrintString` (`KismetStringLibrary.Conv_BoolToString` _isposavailable_)))

(fn `FindPath`
  (params (StartPos :type "Vector Structure") (EndPos :type "Vector Structure"))
  (returns (path :type "Array of Vector Structure"))
  (locals (OpenList :type "Array of Vector Structure") (ClosedList :type "Array of Vector Structure") (F_Array :type "Array of Integer") (currentPos :type "Vector Structure") (OpenListTiles :type "Array of /Game/BluePrintActors/Tiles/BP_Tile Object Reference") (ClosedListTiles :type "Array of /Game/BluePrintActors/Tiles/BP_Tile Object Reference") (Direction :type "Array of Vector Structure") (neighbor :type "Vector Structure"))
  (bind _bp_tilesmanagerref (`self.BP_TilesManagerRef`))
  (bind _openlisttiles (`local.OpenListTiles`))
  (bind _tile (`/Game/BluePrintActors/Managers/BP_TilesManager.GetTileAtPosition` (`self.BP_TilesManagerRef`) StartPos))
  (`KismetArrayLibrary.Array_Add` _openlisttiles _tile)
  (while (> (`KismetArrayLibrary.Array_Length` _openlisttiles) 0)
    (bind _outarray (`self.SortArray` (`local.OpenListTiles`)))
    (bind _output_get (set `local.currentPos` (`SceneComponent.K2_GetComponentLocation` (`/Game/BluePrintActors/Tiles/BP_Tile.CollisonSphere` (`|GetArrayItem` _outarray)))))
    (bind _tile_2 (`/Game/BluePrintActors/Managers/BP_TilesManager.GetTileAtPosition` (`self.BP_TilesManagerRef`) _output_get))
    (`KismetArrayLibrary.Array_RemoveItem` (`local.OpenListTiles`) _tile_2)
    (`KismetArrayLibrary.Array_Add` (`local.ClosedListTiles`) _tile_2)
    (if (== (`local.currentPos`) EndPos)
      (bind _finishereversedlist (`self.Restructure Path` StartPos EndPos))
      (return _finishereversedlist)
      (else
        (for _array_element (`local.Direction`)
          (set `local.neighbor` (+ (`local.currentPos`) _array_element))
          (bind _isposavailable_ (`self.IsPositionAvailable` (`local.neighbor`)))
          (bind _tile_3 (`/Game/BluePrintActors/Managers/BP_TilesManager.GetTileAtPosition` (`self.BP_TilesManagerRef`) (`local.neighbor`)))
          (if (not (or (== _isposavailable_ false) (`KismetArrayLibrary.Array_Contains` (`local.ClosedListTiles`) _tile_3)))
            (bind _tile_4 (`/Game/BluePrintActors/Managers/BP_TilesManager.GetTileAtPosition` _bp_tilesmanagerref (`local.neighbor`)))
            (bind _int (`self.GetMathanttenDistance` StartPos (`local.neighbor`)))
            (set `/Game/BluePrintActors/Tiles/BP_Tile.G` _int _tile_4)
            (bind _tile_5 (`/Game/BluePrintActors/Managers/BP_TilesManager.GetTileAtPosition` _bp_tilesmanagerref (`local.neighbor`)))
            (bind _int_2 (`self.GetMathanttenDistance` EndPos (`local.neighbor`)))
            (set `/Game/BluePrintActors/Tiles/BP_Tile.H` _int_2 _tile_5)
            (bind _tile_6 (`/Game/BluePrintActors/Managers/BP_TilesManager.GetTileAtPosition` _bp_tilesmanagerref (`local.neighbor`)))
            (bind _tile_7 (`/Game/BluePrintActors/Managers/BP_TilesManager.GetTileAtPosition` (`self.BP_TilesManagerRef`) (`local.currentPos`)))
            (set `/Game/BluePrintActors/Tiles/BP_Tile.BP_PreviousTile` _tile_7 _tile_6)
            (bind _tile_8 (`/Game/BluePrintActors/Managers/BP_TilesManager.GetTileAtPosition` (`self.BP_TilesManagerRef`) (`local.neighbor`)))
            (if (not (`KismetArrayLibrary.Array_Contains` (`local.OpenListTiles`) _tile_8))
              (`KismetArrayLibrary.Array_Add` (`local.OpenListTiles`) _tile_8)))))))
  (return))

(fn `FindPathDijkstra`)

(fn `GetAvailableTiles`
  (params (StartPos :type "Vector Structure") (Range :type Integer))
  (returns (AvailableTiles :type "Map of Vector Structure to Integer"))
  (locals (tmpArrayL :type "Array of Vector Structure") (AvailableTilesL :type "Map of Vector Structure to Object Object Reference") (CurrentPosL :type "Vector Structure") (DirectionsL :type "Array of Vector Structure") (NeighborL :type "Vector Structure"))
  (bind _tmparrayl (`local.tmpArrayL`))
  (bind _tmparrayl_2 (`local.tmpArrayL`))
  (`BlueprintMapLibrary.Map_Add` (`local.AvailableTilesL`) StartPos)
  (`KismetArrayLibrary.Array_Add` _tmparrayl_2 StartPos)
  (while (> (`KismetArrayLibrary.Array_Length` _tmparrayl_2) 0)
    (bind _output_get (set `local.CurrentPosL` (`|GetArrayItem` _tmparrayl)))
    (`KismetArrayLibrary.Array_RemoveItem` _tmparrayl _output_get)
    (for _array_element (`local.DirectionsL`)
      (bind _output_get_2 (set `local.NeighborL` (+ (`local.CurrentPosL`) _array_element)))
      (bind _isposavailable_ (`self.IsPositionAvailable` _output_get_2))
      (if (and _isposavailable_ (not (`BlueprintMapLibrary.Map_Contains` (`local.AvailableTilesL`) _output_get_2)))
        (bind _returnvalue (+ (`BlueprintMapLibrary.Map_Find` (`local.AvailableTilesL`) _output_get) 1))
        (if (<= _returnvalue Range)
          (`BlueprintMapLibrary.Map_Add` (`local.AvailableTilesL`) _output_get_2 _returnvalue)
          (`KismetArrayLibrary.Array_Add` (`local.tmpArrayL`) _output_get_2))))
    (`KismetSystemLibrary.PrintString` "Fin "))
  (return (`local.AvailableTilesL`)))

(fn `GetMathanttenDistance`
  (params (StartPos :type "Vector Structure") (neighborPos :type "Vector Structure"))
  (returns (int :type Integer))
  (return (+ (`KismetMathLibrary.Abs_Int` (- (`KismetMathLibrary.FFloor` (.x StartPos)) (`KismetMathLibrary.FFloor` (.x neighborPos)))) (`KismetMathLibrary.Abs_Int` (- (`KismetMathLibrary.FFloor` (.y StartPos)) (`KismetMathLibrary.FFloor` (.y neighborPos)))))))

(fn `IsPositionAvailable`
  (params (position :type "Vector Structure"))
  (returns (`IsPosAvailable?` :type Boolean))
  (return (`KismetArrayLibrary.Array_Contains` (`/Game/BluePrintActors/Managers/BP_TilesManager.TilesPosition` (`self.BP_TilesManagerRef`)) position)))

(fn `Restructure Path`
  (params (StartPos :type "Vector Structure") (EndPos :type "Vector Structure"))
  (returns (FinisheReversedList :type "Array of Vector Structure"))
  (locals (finishedList :type "Array of Vector Structure") (CurrentPos :type "Vector Structure"))
  (set `local.CurrentPos` EndPos)
  (while (!= (`local.CurrentPos`) StartPos)
    (`KismetArrayLibrary.Array_Add` (`local.finishedList`) (`local.CurrentPos`))
    (bind _tile (`/Game/BluePrintActors/Managers/BP_TilesManager.GetTileAtPosition` (`self.BP_TilesManagerRef`) (`local.CurrentPos`)))
    (set `local.CurrentPos` (`SceneComponent.K2_GetComponentLocation` (`/Game/BluePrintActors/Tiles/BP_Tile.CollisonSphere` (`/Game/BluePrintActors/Tiles/BP_Tile.BP_PreviousTile` _tile)))))
  (`KismetArrayLibrary.Array_Reverse` (`local.finishedList`))
  (return (`local.finishedList`)))

(fn `SortArray`
  (params (Tiles :type "Array of /Game/BluePrintActors/Tiles/BP_Tile Object Reference"))
  (returns (OutArray :type "Array of /Game/BluePrintActors/Tiles/BP_Tile Object Reference"))
  (locals (tmpArray :type "Array of /Game/BluePrintActors/Tiles/BP_Tile Object Reference") (`tmp Elements` :type Integer) (`In Array` :type "Array of /Game/BluePrintActors/Tiles/BP_Tile Object Reference") (`Tmp Actor` :type "/Game/BluePrintActors/Tiles/BP_Tile Object Reference") (`Tmp F Distance Array` :type "Array of Integer") (`Tmp Found Index` :type Integer) (`Tmp Out Array` :type "Array of /Game/BluePrintActors/Tiles/BP_Tile Object Reference"))
  (set `local.tmpArray` Tiles)
  (set `local.tmp Elements` (`KismetArrayLibrary.Array_LastIndex` Tiles))
  (bind _arrayelementref (`/Game/Macros/CustomRefLoop.ForEachRefLoop` Tiles)
    (:`Update`
      (bind _output_get (set `local.Tmp Actor` _arrayelementref))
      (bind _output_get_2 (set `/Game/BluePrintActors/Tiles/BP_Tile.F` (+ (`/Game/BluePrintActors/Tiles/BP_Tile.G` _output_get) (`/Game/BluePrintActors/Tiles/BP_Tile.H` _output_get)) _output_get))
      (`KismetArrayLibrary.Array_Add` (`local.Tmp F Distance Array`) _output_get_2))
    (:`Complete`
      (for _ (range (+ (`local.tmp Elements`) 1))
        (bind _output_get_3 (set `local.Tmp Found Index` (`KismetMathLibrary.MinOfIntArray` (`local.Tmp F Distance Array`))))
        (`KismetArrayLibrary.Array_Add` (`local.Tmp Out Array`) (`|GetArrayItem` (`local.tmpArray`) _output_get_3))
        (`KismetArrayLibrary.Array_Remove` (`local.Tmp F Distance Array`) (`local.Tmp Found Index`))
        (`KismetArrayLibrary.Array_Remove` (`local.tmpArray`) (`local.Tmp Found Index`)))
      (return (`local.Tmp Out Array`)))))

(fn `SortArrayByInt`
  (params (`Int Array` :type "Array of Integer") (Tiles :type "Array of /Game/BluePrintActors/Tiles/BP_Tile Object Reference"))
  (returns (Sorted :type "Array of Integer") (SortedOldIndex :type "Array of Integer"))
  (locals (`Array Int Val` :type "Array of Integer") (`Array Old Index` :type "Array of Integer") (`Sorted Array` :type "Array of Integer") (`F_Tiles Array` :type "Array of Integer"))
  (bind _array_int_val (`local.Array Int Val`))
  (bind (_indexofminvalue _minvalue) (`KismetMathLibrary.MinOfIntArray` _array_int_val))
  (for (_array_element _array_index) Tiles
    (`KismetArrayLibrary.Array_Set` (`local.F_Tiles Array`) _array_index (`/Game/BluePrintActors/Tiles/BP_Tile.F` _array_element))
    (for (_array_element_2 _array_index_2) `Int Array`
      (`KismetArrayLibrary.Array_Set` (`local.Array Int Val`) _array_index_2 _array_element_2 true))
    (for _index (range (+ (`KismetArrayLibrary.Array_LastIndex` `Int Array`) 1))
      (`KismetArrayLibrary.Array_Set` (`local.Array Old Index`) _index _indexofminvalue true)
      (`KismetArrayLibrary.Array_Set` (`local.Sorted Array`) _index _minvalue true)
      (`KismetArrayLibrary.Array_Set` _array_int_val _indexofminvalue (+ (`.MaxValue` (`KismetMathLibrary.MaxOfIntArray` `Int Array`)) 1)))
    (return (`local.Sorted Array`) (`local.Array Old Index`))))

(fn `UserConstructionScript`)